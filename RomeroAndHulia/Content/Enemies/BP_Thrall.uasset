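; Thrall enemy character that patrols, shows random dialogue lines and can be taken down by the player.
; Within range of the player, it rebuilds a vision-cone procedural mesh every tick from a fan of line traces, so obstacles clip it.
; Box overlap sets the player's takedown flag and toggles a camera-facing key prompt; TakeDown plays an assassination montage, then destroys the actor.
; Helper functions expose its patrol route and set walk speed.
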(event OnComponentBeginOverlap(Box)
  (params (OverlappedComponent :type Primitive%20Component%20Object%20Reference) (OtherActor :type Actor%20Object%20Reference) (OtherComp :type Primitive%20Component%20Object%20Reference) (OtherBodyIndex :type Integer) (bFromSweep :type Boolean) (SweepResult :type Hit%20Result%20Structure%20%28by%20ref%29))
  ;[0 0.02733 1] Gegner töten
  (bind _asbp_player_top_down (Utilities|Casting|CastToBP_PlayerTopDown OtherActor))
  (Variables|/Game/Player/Blueprints/BP_PlayerTopDown.BP_PlayerTopDown_C|SetCanTakeDown _asbp_player_top_down true)
  (if (Variables|/Game/Player/Blueprints/BP_PlayerTopDown.BP_PlayerTopDown_C|GetVerwandelt _asbp_player_top_down)
    (Development|SetHiddeninGame (Variables|Default|GetTaste) false false)))

(event OnComponentEndOverlap(Box)
  (params (OverlappedComponent :type Primitive%20Component%20Object%20Reference) (OtherActor :type Actor%20Object%20Reference) (OtherComp :type Primitive%20Component%20Object%20Reference) (OtherBodyIndex :type Integer))
  ;[0 0.02733 1] Gegner töten
  (bind _asbp_player_top_down (Utilities|Casting|CastToBP_PlayerTopDown OtherActor))
  (Variables|/Game/Player/Blueprints/BP_PlayerTopDown.BP_PlayerTopDown_C|SetCanTakeDown _asbp_player_top_down false)
  (if (Variables|/Game/Player/Blueprints/BP_PlayerTopDown.BP_PlayerTopDown_C|GetVerwandelt (stale OnComponentBeginOverlap(Box) _asbp_player_top_down))
    (Development|SetHiddeninGame (Variables|Default|GetTaste) true false)))

(event Custom|Dialogue
  (Development|SetHiddeninGame (Variables|Default|GetDialogueText) false false)
  (Rendering|Components|TextRender|SetText (Variables|Default|GetDialogueText) (.OutItem (Utilities|Array|Random (Variables|Default|GetDialogues))))
  (Utilities|FlowControl|Delay 6.0)
  (Development|SetHiddeninGame (Variables|Default|GetDialogueText) true false))

(event Custom|TakeDown
  ;[0 0.02733 1] Gegner töten
  (Pawn|Components|CharacterMovement|DisableMovement (Variables|Character|GetCharacterMovement))
  (Collision|SetActorEnableCollision false)
  (bind _returnvalue (Animation|PlayAnimMontage "/Game/Enemies/Animation/AssassinationEnemy_Montage.AssassinationEnemy_Montage" 1.0 "None"))
  (Utilities|FlowControl|Delay _returnvalue)
  (Actor|DestroyActor))

(event Custom|RotateTextToPlayer
  (bind _dialoguetext (Variables|Default|GetDialogueText))
  (if (not (Variables|/Script/Engine.SceneComponent|GetbHiddenInGame (Variables|Default|GetDialogueText)))
    (Transformation|SetWorldRotation _dialoguetext (Camera|GetCameraRotation (Game|GetPlayerCameraManager 0)) false false)
    (Transformation|AddLocalRotation _dialoguetext "0.000000,-180.000000,0.000000" false false)))

(event Custom|MBPause
  ;[0.01018 0 1] keiner weiß
  (Pawn|Components|CharacterMovement|DisableMovement (Variables|Character|GetCharacterMovement)))

(event Custom|MBResume
  ;[0.01018 0 1] keiner weiß
  (Pawn|Components|CharacterMovement|SetMovementMode (Variables|Character|GetCharacterMovement) "MOVE_NavWalking" 0))

(event Custom|RotateTastenWidget
  (bind _taste (Variables|Default|GetTaste))
  (if (not (Variables|/Script/Engine.SceneComponent|GetbHiddenInGame (Variables|Default|GetTaste)))
    (Transformation|SetWorldRotation _taste (Camera|GetCameraRotation (Game|GetPlayerCameraManager 0)) false false)
    (Transformation|AddLocalRotation _taste "0.000000,-180.000000,0.000000" false false)))

(event EventTick
  (params (DeltaSeconds :type Float%20%28single-precision%29))
  (bind _proceduralmesh (Variables|Default|GetProceduralMesh))
  (CallFunction|RotateTastenWidget)
  (CallFunction|RotateTexttoPlayer)
  (if (<= (Math|Vector|Distance(Vector) (Transformation|GetActorLocation) (Transformation|GetActorLocation (Game|GetPlayerCharacter 0))) (Variables|Default|GetShowVisionCone))
    (if (Variables|/Script/Engine.SceneComponent|GetbHiddenInGame _proceduralmesh)
      (Development|SetHiddeninGame _proceduralmesh false false))
    (CallFunction|Update)
    (CallFunction|LineTracing)
    (else
      (Development|SetHiddeninGame (Variables|Default|GetProceduralMesh) true false))))

(event EventBeginPlay
  (Utilities|Time|SetTimerbyEvent (EventDispatchers|CreateEvent :!event Custom|Dialogue) (Math|Random|RandomFloatinRange 3e+01 6e+01) true))

(fn ConstructionScript
  (if (Variables|VisionArea|GetbRebuild)
    _
    (else
      _))
  (CallFunction|Start)
  (CallFunction|LineTracing))

(fn Start
  (Utilities|FlowControl|Sequence
    (:then_0
      (bind _output_get (Variables|VisionArea|SetNumberOfSection (Math|Float|Ceil (/ (* (Variables|VisionArea|GetHalfAngle) 2.0) (Variables|VisionArea|GetDeltaAngle)))))
      (Variables|VisionArea|SetdAngle (/ (* (Variables|VisionArea|GetHalfAngle) 2.0) _output_get)))
    (:then_1
      (Variables|VisionArea|SetStartPoint (+ (Math|Vector|MakeVector 0.0 0.0 (- (Variables|VisionArea|GetHeightOfCheck) 1e+02)) (Transformation|GetActorLocation))))
    (:then_2
      (Transformation|AddLocalOffset (Variables|Default|GetProceduralMesh) (Math|Vector|MakeVector 0.0 0.0 (- (Variables|VisionArea|GetHeigthOfShow) 1e+02)) false false))))

(fn LineTracing
  (bind _startpoint (Variables|VisionArea|GetStartPoint))
  (for _index (range 0 (Variables|VisionArea|GetNumberOfSection))
    (LocalVariables|SetLCurrentAngle (- (* _index (Variables|VisionArea|GetdAngle)) (Variables|VisionArea|GetHalfAngle)))
    (bind _outhit (Collision|LineTraceByChannel _startpoint (+ _startpoint (* (Math|Vector|RotateVectorAroundAxis (Transformation|GetActorForwardVector) (LocalVariables|GetLCurrentAngle) "0.000000,0.000000,1.000000") (Variables|VisionArea|GetExternalRadius))) "TraceTypeQuery1" false 0 (Variables|VisionArea|GetDrawDebugType) true "(R=1.000000,G=0.000000,B=0.000000,A=1.000000)" "(R=0.000000,G=1.000000,B=0.000000,A=1.000000)" (Variables|VisionArea|GetDrawTime)))
    (Utilities|Array|Add (Variables|VisionArea|GetHitResults) _outhit))
  (CallFunction|CreateProceduralMesh))

(fn CreateProceduralMesh
  (for _index (range 0 (- (Utilities|Array|LastIndex (Variables|VisionArea|GetHitResults)) 1))
    (LocalVariables|Seti _index)
    (Utilities|FlowControl|Sequence
      (:then_0
        (if (.bBlockingHit (Collision|BreakHitResult (Utilities|Array|Get(acopy) (Variables|VisionArea|GetHitResults) (LocalVariables|Geti))))
          (LocalVariables|SetLLeftPoint (.Location (Collision|BreakHitResult (Utilities|Array|Get(acopy) (Variables|VisionArea|GetHitResults) (LocalVariables|Geti)))))
          (else
            (LocalVariables|SetLLeftPoint (.TraceEnd (Collision|BreakHitResult (Utilities|Array|Get(acopy) (Variables|VisionArea|GetHitResults) (LocalVariables|Geti))))))))
      (:then_1
        (if (.bBlockingHit (Collision|BreakHitResult (Utilities|Array|Get(acopy) (Variables|VisionArea|GetHitResults) (+ (LocalVariables|Geti) 1))))
          (LocalVariables|SetLRightPoint (.Location (Collision|BreakHitResult (Utilities|Array|Get(acopy) (Variables|VisionArea|GetHitResults) (+ (LocalVariables|Geti) 1)))))
          (else
            (LocalVariables|SetLRightPoint (.TraceEnd (Collision|BreakHitResult (Utilities|Array|Get(acopy) (Variables|VisionArea|GetHitResults) (+ (LocalVariables|Geti) 1))))))))
      (:then_2
        (Class|ProceduralMeshComponent|CreateMeshSectionLinearColor (Variables|Default|GetProceduralMesh) (LocalVariables|Geti) (Utilities|Array|MakeArray (- (Variables|VisionArea|GetStartPoint) (Variables|VisionArea|GetStartPoint)) (- (LocalVariables|GetLLeftPoint) (Variables|VisionArea|GetStartPoint)) (- (LocalVariables|GetLRightPoint) (Variables|VisionArea|GetStartPoint))) (Utilities|Array|MakeArray 0 2 1) 0 0 0 0 0 0 0 false false)
        (Rendering|Material|SetMaterial (Variables|Default|GetProceduralMesh) (LocalVariables|Geti) "/Game/Enemies/VisionCone/MI_Base.MI_Base"))))
  (Transformation|SetRelativeRotation (Variables|Default|GetProceduralMesh) (* (Math|Rotator|MakeRotfromX (Transformation|GetActorForwardVector)) -1.0) false false))

(fn Update
  (Variables|VisionArea|SetStartPoint (+ (Math|Vector|MakeVector 0.0 0.0 (- (Variables|VisionArea|GetHeightOfCheck) 1e+02)) (Transformation|GetActorLocation)))
  (Utilities|Array|Clear (Variables|VisionArea|GetHitResults))
  (Class|ProceduralMeshComponent|ClearAllMeshSections (Variables|Default|GetProceduralMesh)))

(fn GetPatrolRoute
  (return (Variables|Default|GetPatrolRoute)))

(fn RotatetoTarget
  (return "0, 0, 0"))

(fn SetMovementSpeed
  (params (movementSpeed :type E_movementSpeed%20Enum :default "NewEnumerator0"))
  (bind _output_get (Variables|/Script/Engine.CharacterMovementComponent|SetMaxWalkSpeed (Variables|Character|GetCharacterMovement) (Utilities|Select :Index movementSpeed :NewEnumerator0 0.0 :NewEnumerator1 1e+02 :NewEnumerator2 3e+02 :NewEnumerator3 5e+02)))
  (return _output_get))