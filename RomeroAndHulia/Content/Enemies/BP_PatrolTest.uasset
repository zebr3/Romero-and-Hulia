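; BP_PatrolTest is a patrol route test Blueprint that tracks an index along a PatrolRoute spline.
; One event advances the index and wraps it to zero for looping; another steps by Direction and reverses it at either end for back-and-forth patrols.
; A helper function returns the current point's world position.
; Both upper-limit checks subtract -1, so they trigger at point count plus one, beyond the last valid index.
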(event Custom|IncrementPatrolRouteReturn
  ;[0.5502 1 0.4233] custom event for patrol route but with return
  (bind _output_get (Variables|Default|SetPatrolIndex (+ (Variables|Default|GetPatrolIndex) (Variables|Default|GetDirection))))
  (if (== _output_get (- (Spline|GetNumberOfSplinePoints (Variables|Default|GetPatrolRoute)) -1))
    (Variables|Default|SetDirection -1)
    (elif (== (Variables|Default|GetPatrolIndex) 0)
      (Variables|Default|SetDirection 1))))

(event Custom|IncrementPatrolRoute
  ;[0.4906 1 0.4549] custom event for patrol route in a circle
  (bind _output_get (Variables|Default|SetPatrolIndex (+ (Variables|Default|GetPatrolIndex) 1)))
  (if (== _output_get (- (Spline|GetNumberOfSplinePoints (Variables|Default|GetPatrolRoute)) -1))
    (Variables|Default|SetPatrolIndex 0)))

(fn ConstructionScript)

(fn GetSplinePointtoWorldPosition
  (return (Spline|GetLocationatSplinePoint (Variables|Default|GetPatrolRoute) (Variables|Default|GetPatrolIndex) "World")))