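; Item data component that makes its owning actor a pickup for the player's inventory.
; On interaction it passes its item row name and quantity to the player character's inventory component, then destroys the owner if the add succeeds.
; LookAt returns an empty string, and a SetReplicates call on the owner is left unconnected, so it never runs.
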(event EventBeginPlay
  ;[0 0.1298 1] für multiplayer idk lol
)

(event EventInteractwith
  (params (PlayerCharacter :type BP%20Player%20Top%20Down%20Object%20Reference))
  (bind _bpc_inventorysystem (Variables|/Game/Player/Blueprints/BP_PlayerTopDown.BP_PlayerTopDown_C|GetBPC_InventorySystem PlayerCharacter))
  (Utilities|IsValid _bpc_inventorysystem
    (:Is%20Valid
      (bind _success (Default|AddtoInventory _bpc_inventorysystem (.rowname (Variables|Default|GetItemID)) (Variables|Default|GetQuantity)))
      (if _success
        (Actor|DestroyActor (Components|GetOwner))))))

(fn Lookat
  (return ""))