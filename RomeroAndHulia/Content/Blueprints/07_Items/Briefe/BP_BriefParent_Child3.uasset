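; Third letter ("Brief") pickup item, which by its name is a child of BP_BriefParent.
; When the IA_PickUp input action completes, it creates the WB_Brief3 widget, adds it to the viewport, then destroys itself after a short delay.
; It has no range or overlap check of its own; its BeginPlay, overlap and Tick events are unused stubs and its construction script just calls the parent.
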(event Input|EnhancedActionEvents|EnhancedInputActionIA_PickUp
  (params (ActionValue :type Boolean) (ElapsedSeconds :type Float%20%28double-precision%29) (TriggeredSeconds :type Float%20%28double-precision%29) (InputAction :type Input%20Action%20Object%20Reference :default "/Game/Player/Input/Actions/IA_PickUp.IA_PickUp"))
  (:Completed
    (bind _returnvalue (UserInterface|CreateWidget "/Game/UI/WB_Brief3.WB_Brief3_C"))
    (UserInterface|Viewport|AddtoViewport _returnvalue 0)
    (Utilities|FlowControl|Delay 1.0)
    (Actor|DestroyActor)))

(event EventBeginPlay
  (|CallParentFunction) ; This node is disabled and will not be called.\nDrag off pins to build functionality.
)

(event Collision|EventActorBeginOverlap
  (params (OtherActor :type Actor%20Object%20Reference))
  (|CallParentFunction OtherActor) ; This node is disabled and will not be called.\nDrag off pins to build functionality.
)

(event EventTick
  (params (DeltaSeconds :type Float%20%28single-precision%29))
  (|CallParentFunction DeltaSeconds) ; This node is disabled and will not be called.\nDrag off pins to build functionality.
)

(fn ConstructionScript
  (|CallParentFunction))