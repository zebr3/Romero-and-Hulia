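; BP_Item is a world item that the player can pick up, showing a text label and supplying a pickup prompt.
; Sphere2 overlaps with BP_PlayerTopDown toggle the label's visibility, and Tick keeps it turned toward the camera.
; LookAt builds the "Pick up" prompt from the item's data table row, via ItemDataComponent.
; PickUpItem returns the Item and triggers destruction of the actor after a short delay.
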(event OnComponentBeginOverlap(Sphere2)
  (params (OverlappedComponent :type Primitive%20Component%20Object%20Reference) (OtherActor :type Actor%20Object%20Reference) (OtherComp :type Primitive%20Component%20Object%20Reference) (OtherBodyIndex :type Integer) (bFromSweep :type Boolean) (SweepResult :type Hit%20Result%20Structure%20%28by%20ref%29))
  (Utilities|Casting|CastToBP_PlayerTopDown OtherActor)
  (Rendering|ToggleVisibility (Variables|Default|GetTextRender) false))

(event OnComponentEndOverlap(Sphere2)
  (params (OverlappedComponent :type Primitive%20Component%20Object%20Reference) (OtherActor :type Actor%20Object%20Reference) (OtherComp :type Primitive%20Component%20Object%20Reference) (OtherBodyIndex :type Integer))
  (Utilities|Casting|CastToBP_PlayerTopDown OtherActor)
  (Rendering|ToggleVisibility (Variables|Default|GetTextRender) false))

(event Custom|Destroy%20Item
  (Utilities|FlowControl|Delay 0.1)
  (Actor|DestroyActor))

(event EventTick
  (params (DeltaSeconds :type Float%20%28single-precision%29))
  (bind _textrender (Variables|Default|GetTextRender))
  (Transformation|SetWorldRotation _textrender (.Rotation (Math|Transform|BreakTransform (Transformation|GetActorTransform (Game|GetPlayerCameraManager 0)))) false false)
  (Transformation|AddLocalRotation _textrender "0.000000,-180.000000,0.000000" false false))

(fn ConstructionScript)

(fn Lookat
  (bind _itemdatacomponent (Variables|Default|GetItemDataComponent))
  (bind _itemid (Variables|/Game/Blueprints/08_Inventory/ItemDataComponent.ItemDataComponent_C|GetItemID _itemdatacomponent))
  (bind _returnvalue (Utilities|GetDataTableRow (.datatable _itemid) (.rowname _itemid))
    (:then
      (return (Utilities|Text|FormatText "Pick up {item}" (.Name (Utilities|Struct|BreakFItemStruct _returnvalue)))))))

(fn PickUpItem
  (CallFunction|DestroyItem)
  (return (Variables|Default|GetItem)))