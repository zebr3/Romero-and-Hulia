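; BP_Hebel is a lever that the player toggles with F inside its trigger box to operate the secret door.
; A FlipFlop plays or reverses a Timeline that rotates the lever mesh.
; When the Timeline finishes, it finds BP_SecretTür, plays a sound and calls TürAuf.
; The first time, it also spawns blood explosions and a gore sound, then calls ChangeMesh after a delay, guarded by KerkerTypSchonTot.
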(event OnComponentBeginOverlap(Box)
  (params (OverlappedComponent :type Primitive%20Component%20Object%20Reference) (OtherActor :type Actor%20Object%20Reference) (OtherComp :type Primitive%20Component%20Object%20Reference) (OtherBodyIndex :type Integer) (bFromSweep :type Boolean) (SweepResult :type Hit%20Result%20Structure%20%28by%20ref%29))
  (Utilities|Casting|CastToBP_PlayerTopDown OtherActor)
  (Input|EnableInput (Game|GetPlayerController 0)))

(event OnComponentEndOverlap(Box)
  (params (OverlappedComponent :type Primitive%20Component%20Object%20Reference) (OtherActor :type Actor%20Object%20Reference) (OtherComp :type Primitive%20Component%20Object%20Reference) (OtherBodyIndex :type Integer))
  (Utilities|Casting|CastToBP_PlayerTopDown OtherActor)
  (Input|DisableInput (Game|GetPlayerController 0)))

(event Input|EnhancedActionEvents|EnhancedInputActionIA_PickUp
  (params (ActionValue :type Boolean) (ElapsedSeconds :type Float%20%28double-precision%29) (TriggeredSeconds :type Float%20%28double-precision%29) (InputAction :type Input%20Action%20Object%20Reference :default "/Game/Player/Input/Actions/IA_PickUp.IA_PickUp")))

(event Input|KeyboardEvents|F
  (params (Key :type Key%20Structure :default "None"))
  (:Released
    (Utilities|FlowControl|FlipFlop
      (:A
        (bind _newtrack_0 (Timeline|Timeline Play)
          (:Update
            (Transformation|SetRelativeRotation (Variables|Default|GetHebel__2__Hebel) (Math|Rotator|MakeRotator 0.0 _newtrack_0 0.0) false false))
          (:Finished
            (bind _returnvalue (Actor|GetActorOfClass "/Game/Blueprints/09_SecretTür/BP_SecretTür.BP_SecretTür_C"))
            (Utilities|IsValid _returnvalue
              (:Is%20Valid
                (Audio|PlaySoundatLocation "/Game/Sound/Soundeffects/Items/Hebel.Hebel" (Transformation|GetActorLocation) "0, 0, 0" 1.0 1.0 0.0 "/Game/Sound/SoundAttenuationStandard.SoundAttenuationStandard" 0 0 0)
                (bind _output_get (Variables|Default|SetSecretTür _returnvalue))
                (if (Variables|Default|GetKerkerTypSchonTot?)
                  (Default|TürAuf _output_get)
                  (else
                    (Niagara|SpawnSystematLocation "/Game/VFX/Niagra/NS_Bloodexplosion.NS_Bloodexplosion" (+ (Transformation|GetWorldLocation (Variables|/Game/Blueprints/09_SecretTür/BP_SecretTür.BP_SecretTür_C|GetKerkerTypTür _output_get)) "0.000000,0.000000,200.000000"))
                    (Niagara|SpawnSystematLocation "/Game/VFX/Niagra/NS_Bloodexplosion.NS_Bloodexplosion" (+ (Transformation|GetWorldLocation (Variables|/Game/Blueprints/09_SecretTür/BP_SecretTür.BP_SecretTür_C|GetKerkerTypTot (Variables|Default|GetSecretTür))) "150.000000,90.000000,0.000000"))
                    (Audio|PlaySoundatLocation "/Game/Sound/Soundeffects/Enemy/DudeWirdZerrissen.DudeWirdZerrissen" (Transformation|GetActorLocation (Variables|Default|GetSecretTür)) "0, 0, 0" 1.0 1.0 0.0 "/Game/Sound/SoundAttenuationStandard.SoundAttenuationStandard" 0 0 0)
                    (Default|TürAuf (Variables|Default|GetSecretTür))
                    (Utilities|FlowControl|Delay 1.2)
                    (Default|ChangeMesh (Variables|Default|GetSecretTür))))
                (Variables|Default|SetKerkerTypSchonTot? true))))))
      (:B
        (Timeline|Timeline Reverse)))))

(fn ConstructionScript)