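; Secret rear double door that slides its two panels apart and back whenever the TürAuf event is called.
; A FlipFlop alternates between playing and reversing one Timeline, whose track sets the relative X of the right panel and the negated value for the left.
; An older world-location variant for the right panel remains in the graph but never runs.
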(event Custom|TürAuf
  (Utilities|FlowControl|FlipFlop
    (:A
      (bind _newtrack_0 (Timeline|Timeline Play)
        (:Update
          (Transformation|SetRelativeLocation (Variables|Default|GetSecretTürRechts) (Math|Vector|MakeVector _newtrack_0 0.0 0.0) false false)
          (Transformation|SetRelativeLocation (Variables|Default|GetSecretTürLinks) (* (Math|Vector|MakeVector _newtrack_0 0.0 0.0) "-1.000000,0.000000,0.000000") false false))))
    (:B
      (Timeline|Timeline Reverse))))

(event EventBeginPlay)

(event Collision|EventActorBeginOverlap
  (params (OtherActor :type Actor%20Object%20Reference)))

(event EventTick
  (params (DeltaSeconds :type Float%20%28single-precision%29)))

(fn ConstructionScript)