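; Secret door actor that slides two panels apart or back on alternate triggers and includes a dungeon character with alive and dead states.
; A timeline mirrors both panels' movement and plays a one-time "torn apart" sound on the first opening.
; ChangeMesh toggles the character and shackle meshes and marks it dead, which silences Dialogue's random, briefly shown lines.
; Tick turns visible text toward the camera, while BeginPlay starts a looping, randomly timed timer.
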(event Custom|Dialogue
  (if (not (Variables|Default|Gettot))
    (Development|SetHiddeninGame (Variables|Default|GetTextRender) false false)
    (Rendering|Components|TextRender|SetText (Variables|Default|GetTextRender) (.OutItem (Utilities|Array|Random (Variables|Default|GetDialogues))))
    (Utilities|FlowControl|Delay 6.0)
    (Development|SetHiddeninGame (Variables|Default|GetTextRender) true false)))

(event Custom|Change%20Mesh
  (Rendering|ToggleVisibility (Variables|Default|GetKerkerTypTür) false)
  (Rendering|ToggleVisibility (Variables|Default|GetKerkerTypTot) false)
  (Rendering|ToggleVisibility (Variables|Default|GetKerker_WachraumÜberarbeitet_Fesseln_003) false)
  (Rendering|ToggleVisibility (Variables|Default|GetKerker_WachraumÜberarbeitet_Fesseln_004) false)
  (Variables|Default|Settot true))

(event Custom|RotateTextToPlayer
  (bind _textrender (Variables|Default|GetTextRender))
  (if (not (Variables|/Script/Engine.SceneComponent|GetbHiddenInGame _textrender))
    (Transformation|SetWorldRotation _textrender (Camera|GetCameraRotation (Game|GetPlayerCameraManager 0)) false false)
    (Transformation|AddLocalRotation _textrender "0.000000,-180.000000,0.000000" false false)))

(event Custom|TürAuf
  (Utilities|FlowControl|FlipFlop
    (:A
      (bind _newtrack_0 (Timeline|Timeline Play)
        (:Update
          (Transformation|SetRelativeLocation (Variables|Default|GetSecretTürRechts) (Math|Vector|MakeVector _newtrack_0 0.0 0.0) false false)
          (Transformation|SetRelativeLocation (Variables|Default|GetSecretTürLinks) (* (Math|Vector|MakeVector _newtrack_0 0.0 0.0) "-1.000000,0.000000,0.000000") false false)
          (Utilities|FlowControl|DoOnce false
            (:Completed
              (Audio|PlaySoundatLocation "/Game/Sound/Soundeffects/Enemy/DudeWirdZerrissen.DudeWirdZerrissen" (* (Math|Vector|MakeVector _newtrack_0 0.0 0.0) "-1.000000,0.000000,0.000000") "0, 0, 0" 1.0 1.0 0.0 0 0 0 0))))))
    (:B
      (Timeline|Timeline Reverse))))

(event EventBeginPlay
  (Utilities|Time|SetTimerbyEvent (EventDispatchers|CreateEvent :!event Custom|Dialogue) (Math|Random|RandomFloatinRange 1e+01 2e+01) true))

(event Collision|EventActorBeginOverlap
  (params (OtherActor :type Actor%20Object%20Reference)))

(event EventTick
  (params (DeltaSeconds :type Float%20%28single-precision%29))
  (CallFunction|RotateTexttoPlayer))

(fn ConstructionScript)