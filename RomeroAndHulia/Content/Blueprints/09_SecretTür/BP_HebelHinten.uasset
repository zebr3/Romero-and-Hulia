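; Lever actor that the player flips with the F key to trigger the rear secret door.
; A box overlap with BP_PlayerTopDown enables input on the lever and disables it on exit.
; A FlipFlop alternately plays and reverses a Timeline that drives the handle's pitch rotation.
; When the Timeline finishes, it looks up BP_SecretTürHinten by class and calls TürAuf on it.
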(event OnComponentBeginOverlap(Box)
  (params (OverlappedComponent :type Primitive%20Component%20Object%20Reference) (OtherActor :type Actor%20Object%20Reference) (OtherComp :type Primitive%20Component%20Object%20Reference) (OtherBodyIndex :type Integer) (bFromSweep :type Boolean) (SweepResult :type Hit%20Result%20Structure%20%28by%20ref%29))
  (Utilities|Casting|CastToBP_PlayerTopDown OtherActor)
  (Input|EnableInput (Game|GetPlayerController 0)))

(event OnComponentEndOverlap(Box)
  (params (OverlappedComponent :type Primitive%20Component%20Object%20Reference) (OtherActor :type Actor%20Object%20Reference) (OtherComp :type Primitive%20Component%20Object%20Reference) (OtherBodyIndex :type Integer))
  (Utilities|Casting|CastToBP_PlayerTopDown OtherActor)
  (Input|DisableInput (Game|GetPlayerController 0)))

(event Input|EnhancedActionEvents|EnhancedInputActionIA_PickUp
  (params (ActionValue :type Boolean) (ElapsedSeconds :type Float%20%28double-precision%29) (TriggeredSeconds :type Float%20%28double-precision%29) (InputAction :type Input%20Action%20Object%20Reference :default "/Game/Player/Input/Actions/IA_PickUp.IA_PickUp")))

(event Input|KeyboardEvents|F
  (params (Key :type Key%20Structure))
  (:Pressed
    (Utilities|FlowControl|FlipFlop
      (:A
        (bind _newtrack_0 (Timeline|Timeline Play)
          (:Update
            (Transformation|SetRelativeRotation (Variables|Default|GetHebel__2__Hebel) (Math|Rotator|MakeRotator 0.0 _newtrack_0 0.0) false false))
          (:Finished
            (bind _returnvalue (Actor|GetActorOfClass "/Game/Blueprints/09_SecretTür/BP_SecretTürHinten.BP_SecretTürHinten_C"))
            (Utilities|IsValid _returnvalue
              (:Is%20Valid
                (bind _output_get (Variables|Default|SetNewVar_0 _returnvalue))
                (Default|TürAuf _output_get))))))
      (:B
        (Timeline|Timeline Reverse)))))

(fn ConstructionScript)