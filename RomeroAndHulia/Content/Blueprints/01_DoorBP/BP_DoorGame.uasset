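; BP_DoorGame is a key-locked double door that a top-down player opens and closes with the pick-up input.
; Its box overlap records whether BP_PlayerTopDown has a key and enables input on the door, disabling it when the player leaves.
; With a key, each press alternates a timeline forward and backward, yawing the two gate meshes in opposite directions.
; Without one, it calls the player's DoorKeyText.
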(event OnComponentBeginOverlap(Box)
  (params (OverlappedComponent :type Primitive%20Component%20Object%20Reference) (OtherActor :type Actor%20Object%20Reference) (OtherComp :type Primitive%20Component%20Object%20Reference) (OtherBodyIndex :type Integer) (bFromSweep :type Boolean) (SweepResult :type Hit%20Result%20Structure%20%28by%20ref%29))
  (bind _asbp_player_top_down (Utilities|Casting|CastToBP_PlayerTopDown OtherActor))
  (bind _output_get (Variables|Default|SetAs%20BP%20Player%20Top%20Down _asbp_player_top_down))
  (if (Variables|/Game/Player/Blueprints/BP_PlayerTopDown.BP_PlayerTopDown_C|GetHasKey _output_get)
    (Variables|Default|SetDoorHasKEy true)
    (else
      (Variables|Default|SetDoorHasKEy false)))
  (Input|EnableInput (Game|GetPlayerController 0)))

(event OnComponentEndOverlap(Box)
  (params (OverlappedComponent :type Primitive%20Component%20Object%20Reference) (OtherActor :type Actor%20Object%20Reference) (OtherComp :type Primitive%20Component%20Object%20Reference) (OtherBodyIndex :type Integer))
  (bind _asbp_player_top_down (Utilities|Casting|CastToBP_PlayerTopDown OtherActor))
  (if (Variables|/Game/Player/Blueprints/BP_PlayerTopDown.BP_PlayerTopDown_C|GetHasKey _asbp_player_top_down)
    (Variables|Default|SetDoorHasKEy true)
    (else
      (Variables|Default|SetDoorHasKEy false)))
  (Input|DisableInput (Game|GetPlayerController 0)))

(event Input|EnhancedActionEvents|EnhancedInputActionIA_PickUp
  (params (ActionValue :type Boolean) (ElapsedSeconds :type Float%20%28double-precision%29) (TriggeredSeconds :type Float%20%28double-precision%29) (InputAction :type Input%20Action%20Object%20Reference :default "/Game/Player/Input/Actions/IA_PickUp.IA_PickUp"))
  (:Completed
    (if (Variables|Default|GetDoorHasKEy)
      (Utilities|FlowControl|FlipFlop
        (:A
          (bind _newtrack_0 (Timeline|DoorRotateTimeline Play)
            (:Update
              (Transformation|SetRelativeRotation (Variables|Default|GetTorGizmo_TorRechts) (Math|Rotator|MakeRotator 0.0 0.0 _newtrack_0) false false)
              (Transformation|SetRelativeRotation (Variables|Default|GetTorGizmo_TorLinks) (* (Math|Rotator|MakeRotator 0.0 0.0 _newtrack_0) -1.0) false false))))
        (:B
          (Timeline|DoorRotateTimeline Reverse)))
      (else
        (Default|DoorKeyText (Variables|Default|GetAs%20BP%20Player%20Top%20Down))))))

(fn ConstructionScript)