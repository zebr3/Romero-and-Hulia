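; BP_Schüttelspeer is a talkable actor that shows a sequence of dialogue lines with the wolf portrait.
; Each Talk call types the current line into WB_Dialogue character by character through a short Delay loop, then advances TalkIndex.
; Creating the widget locks the top-down player's camera movement and disables its controller.
; A call after the last line removes the widget and restores both.
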(event EventBeginPlay)

(event Collision|EventActorBeginOverlap
  (params (OtherActor :type Actor%20Object%20Reference)))

(event EventTick
  (params (DeltaSeconds :type Float%20%28single-precision%29)))

(event EventTalk
  (if (< (Variables|Default|GettalkIndex) (Utilities|Array|Length (Variables|Default|Getdialogues)))
    (Variables|Default|GetUI
      (:then
        _)
      (:else
        (bind _returnvalue (UserInterface|CreateWidget "/Game/UI/WB_Dialogue.WB_Dialogue_C"))
        (bind _output_get (Variables|Default|SetUI _returnvalue))
        (UserInterface|Viewport|AddtoViewport _output_get 0)
        (Variables|/Script/UMG.Widget|SetVisibility (Variables|/Game/UI/WB_Dialogue.WB_Dialogue_C|Getwolfportrait (Variables|Default|GetUI)) "Visible")
        (bind _asbp_player_top_down (Utilities|Casting|CastToBP_PlayerTopDown (Game|GetPlayerCharacter 0)))
        (Variables|/Game/Player/Blueprints/BP_PlayerTopDown.BP_PlayerTopDown_C|SetallowCameraMove _asbp_player_top_down false)
        (bind _asbp_top_down_controller (Utilities|Casting|CastToBP_TopDownController (Game|GetPlayerController 0)))
        (Variables|/Game/TopDown/Blueprints/BP_TopDownController.BP_TopDownController_C|Setdisable _asbp_top_down_controller true)))
    (Variables|/Script/UMG.TextBlock|SetText (Variables|/Game/UI/WB_Dialogue.WB_Dialogue_C|GetTextBlock_13 (Variables|Default|GetUI)) "")
    (bind _output_get_2 (Variables|/Script/UMG.TextBlock|SetText (Variables|/Game/UI/WB_Dialogue.WB_Dialogue_C|GetTextBlock_13 (Variables|Default|GetUI)) (Utilities|Text|ToText(String) (Utilities|String|GetSubstring (Utilities|String|ToString(Text) (Utilities|Array|Get(acopy) (Variables|Default|Getdialogues) (Variables|Default|GettalkIndex))) 0 (+ (Utilities|String|Len (Utilities|String|ToString(Text) (Variables|/Script/UMG.TextBlock|GetText (Variables|/Game/UI/WB_Dialogue.WB_Dialogue_C|GetTextBlock_13 (Variables|Default|GetUI))))) 1))) :!label _label))
    (if (Utilities|Enum|Equal(Enum) (Utilities|String|ToString(Text) _output_get_2) (Utilities|String|ToString(Text) (Utilities|Array|Get(acopy) (Variables|Default|Getdialogues) (Variables|Default|GettalkIndex))))
      (Math|Integer|IncrementInt (Variables|Default|GettalkIndex))
      (else
        (Utilities|FlowControl|Delay 0.005)
        (goto _label)))
    (else
      (Widget|RemovefromParent (Variables|Default|GetUI))
      (bind _asbp_player_top_down_2 (Utilities|Casting|CastToBP_PlayerTopDown (Game|GetPlayerCharacter 0)))
      (Variables|/Game/Player/Blueprints/BP_PlayerTopDown.BP_PlayerTopDown_C|SetallowCameraMove _asbp_player_top_down_2 true)
      (bind _asbp_top_down_controller_2 (Utilities|Casting|CastToBP_TopDownController (Game|GetPlayerController 0)))
      (Variables|/Game/TopDown/Blueprints/BP_TopDownController.BP_TopDownController_C|Setdisable _asbp_top_down_controller_2 false))))

(fn ConstructionScript)