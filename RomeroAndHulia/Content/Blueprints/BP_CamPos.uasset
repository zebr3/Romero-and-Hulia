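; BP_CamPos is an actor, likely a camera position anchor by its name, that stays confined to a fixed rectangular area of the world.
; Every Tick, a four-branch sequence checks its location against hardcoded minimum and maximum bounds on X and Y.
; Any out-of-range axis is snapped back to its limit with SetActorLocation, while Z is left unchanged.
; The Blueprint contains no movement logic of its own, only this clamp.
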(event EventTick
  (params (DeltaSeconds :type Float%20%28single-precision%29))
  (bind _returnvalue (Transformation|GetActorLocation))
  (bind _returnvalue_2 (Transformation|GetActorLocation))
  (bind _returnvalue_3 (Transformation|GetActorLocation))
  (bind _returnvalue_4 (Transformation|GetActorLocation))
  (Utilities|FlowControl|Sequence
    (:then_0
      (if (<= (.y _returnvalue_2) 1e+03)
        (Transformation|SetActorLocation (Math|Vector|MakeVector (.x _returnvalue_2) 1e+03 (.z _returnvalue_2)) false false)))
    (:then_1
      (if (>= (.y _returnvalue_3) 1.18e+04)
        (Transformation|SetActorLocation (Math|Vector|MakeVector (.x _returnvalue_3) 1.18e+04 (.z _returnvalue_3)) false false)))
    (:then_2
      (if (<= (.x _returnvalue_4) -4.6e+03)
        (Transformation|SetActorLocation (Math|Vector|MakeVector -4.6e+03 (.y _returnvalue_4) (.z _returnvalue_4)) false false)))
    (:then_3
      (if (>= (.x _returnvalue) 7.2e+03)
        (Transformation|SetActorLocation (Math|Vector|MakeVector 7.2e+03 (.y _returnvalue) (.z _returnvalue)) false false)))))

(fn ConstructionScript)