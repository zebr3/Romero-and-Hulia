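; Test player character Blueprint with werewolf transformation, assassination takedown, cursor teleport, physics knockdown and health bar creation.
; Transforming swaps the mesh and enables a forward-trace takedown on BP_EnemyBase, which snaps behind the enemy, plays a montage, reverts the mesh and grants teleport.
; Teleport, also granted by T, toggles aiming on key 1, then validates a cursor trace with an obstruction trace before a delayed move.
; Hits briefly ragdoll the mesh.
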(event Custom|CreateHealtBarEvent
  ;[0.04774 0.0511 1] erstes Tutorial random shit
  (bind _returnvalue (UserInterface|CreateWidget "/Game/Blueprints/03_DamageBox/WBP_HealthBar.WBP_HealthBar_C" (Game|GetPlayerController 0)))
  (UserInterface|Viewport|AddtoViewport _returnvalue 0))

(event Custom|HitByHitActor
  (params (HitLocation :type Vector))
  (bind _returnvalue (* HitLocation 5e+04))
  (bind (_x _y) (Math|Vector|BreakVector _returnvalue))
  ;[0.04774 0.0511 1] erstes Tutorial random shit
  (if (not (Variables|Default|GetIsKnockedOut))
    (Variables|Default|SetIsKnockedOut true)
    (Physics|SetSimulatePhysics (Variables|Character|GetMesh) true)
    (Physics|AddImpulse (Variables|Character|GetMesh) (Math|Vector|MakeVector _x _y 5e+04) "None" false)
    (Pawn|Components|CharacterMovement|DisableMovement (Variables|Character|GetCharacterMovement))
    (Utilities|FlowControl|Delay 5.0)
    (Physics|SetSimulatePhysics (Variables|Character|GetMesh) false)
    (Transformation|AttachComponentToComponent (Variables|Character|GetMesh) (Variables|Collision|GetCapsuleComponent) "None" "SnapToTarget" "SnapToTarget" "KeepRelative" true)
    (Transformation|SetRelativeLocation (Variables|Character|GetMesh) "0.000000,0.000000,-89.000000" false false)
    (Transformation|SetRelativeRotation (Variables|Character|GetMesh) "0.000000,260.000000,0.000000" false false)
    (Pawn|Components|CharacterMovement|SetMovementMode (Variables|Character|GetCharacterMovement) "MOVE_Walking" 0)
    (Variables|Default|SetIsKnockedOut false)))

(event Custom|ResetKey1
  (bind _cylinder (Variables|Default|GetCylinder))
  ;[0.1075 0.08636 1] Teleport
  (Utilities|FlowControl|FlipFlop
    (:A
      (Rendering|ToggleVisibility _cylinder false)
      (Variables|Default|SetCanTeleport true))
    (:B
      (Rendering|ToggleVisibility _cylinder false)
      (Variables|Default|SetCanTeleport false))))

(event Input|EnhancedActionEvents|EnhancedInputActionIA_TakeDown
  (params (ActionValue :type Boolean) (ElapsedSeconds :type Float%20%28double-precision%29) (TriggeredSeconds :type Float%20%28double-precision%29) (InputAction :type Input%20Action%20Object%20Reference :default "/Game/Player/Input/Actions/IA_TakeDown.IA_TakeDown"))
  (bind _returnvalue (Transformation|GetActorLocation))
  ;[0.08121 0.1267 1] Gegner töten
  (:Completed
    (if (Variables|Default|GetCanVerwandeln)
      (if (Variables|Default|GetCanTakeDown)
        (bind (_outhit _returnvalue_2) (Collision|LineTraceByChannel _returnvalue (+ _returnvalue (* (Transformation|GetActorForwardVector) 2.5e+02)) "TraceTypeQuery1" false 0 "ForDuration"))
        (if _returnvalue_2
          (bind _asbp_enemy_base (Utilities|Casting|CastToBP_EnemyBase (.HitActor (Collision|BreakHitResult _outhit))))
          (Variables|Default|SetAs%20BP%20Enemy%20Base _asbp_enemy_base)
          (Pawn|Components|CharacterMovement|DisableMovement (Variables|Character|GetCharacterMovement))
          (Variables|Default|SetCanTakeDown false)
          (Transformation|SetActorTransform (Math|Transform|MakeTransform (+ (.location (Transformation|GetActorTransform (Variables|Default|GetAs%20BP%20Enemy%20Base))) (* (Transformation|GetActorForwardVector (Variables|Default|GetAs%20BP%20Enemy%20Base)) -175.0)) (.rotation (Transformation|GetActorTransform (Variables|Default|GetAs%20BP%20Enemy%20Base))) "1.000000,1.000000,1.000000"))
          (bind _returnvalue_3 (Animation|PlayAnimMontage "/Game/Enemies/Animation/AssassinationAttacker_Montage.AssassinationAttacker_Montage" 1.0 "None"))
          (Default|TakeDown (Variables|Default|GetAs%20BP%20Enemy%20Base))
          (Utilities|FlowControl|Delay (+ _returnvalue_3 0.025))
          (Transformation|SetActorLocation (+ (Transformation|GetActorLocation) (* (Transformation|GetActorForwardVector) 175.0)) false false)
          (Pawn|Components|CharacterMovement|SetMovementMode (Variables|Character|GetCharacterMovement) "MOVE_Walking" 0)
          (Variables|Default|SetHasTeleportAbility true)
          (Variables|Default|SetCanVerwandeln false)
          (Components|SkeletalMesh|SetSkeletalMeshAsset (Variables|Character|GetMesh) "/Game/Characters/Mannequin_UE4/Meshes/SK_Mannequin.SK_Mannequin"))))))

(event Input|EnhancedActionEvents|EnhancedInputActionIA_Verwandlung
  (params (ActionValue :type Boolean) (ElapsedSeconds :type Float%20%28double-precision%29) (TriggeredSeconds :type Float%20%28double-precision%29) (InputAction :type Input%20Action%20Object%20Reference :default "/Game/Player/Input/Actions/IA_Verwandlung.IA_Verwandlung"))
  (:Completed
    (Variables|Default|SetCanVerwandeln true)
    (Pawn|Components|CharacterMovement|DisableMovement (Variables|Character|GetCharacterMovement))
    (Utilities|FlowControl|Delay 1.5)
    (Components|SkeletalMesh|SetSkeletalMeshAsset (Variables|Character|GetMesh) "/Game/Characters/Mannequin_UE4/Meshes/SK_MannequinWerewolf.SK_MannequinWerewolf")
    (Pawn|Components|CharacterMovement|SetMovementMode (Variables|Character|GetCharacterMovement) "MOVE_Walking" 0)))

(event EventBeginPlay)

(event Input|KeyboardEvents|T
  (params (Key :type Key%20Structure :default "None"))
  ;[0.1075 0.08636 1] Teleport
  (:Pressed
    (Variables|Default|SetHasTeleportAbility true)))

(event Input|KeyboardEvents|1
  (params (Key :type Key%20Structure :default "None"))
  (bind _cylinder (Variables|Default|GetCylinder))
  ;[0.1075 0.08636 1] Teleport
  (:Pressed
    (if (Variables|Default|GetHasTeleportAbility)
      (Utilities|FlowControl|FlipFlop
        (:A
          (Rendering|ToggleVisibility _cylinder false)
          (Variables|Default|SetCanTeleport true))
        (:B
          (Rendering|ToggleVisibility _cylinder false)
          (Variables|Default|SetCanTeleport false))))))

(event Input|MouseEvents|RightMouseButton
  (params (Key :type Key%20Structure :default "None"))
  (bind _returnvalue (Game|GetPlayerController 0))
  (bind (_worldlocation _worlddirection) (Game|Player|ConvertMouseLocationToWorldSpace _returnvalue))
  ;[0.1075 0.08636 1] Teleport
  (:Pressed
    (if (Variables|Default|GetCanTeleport)
      (bind (_outhit _returnvalue_2) (Collision|LineTraceByChannel (- _worldlocation "") (+ _worldlocation (* _worlddirection 4e+03)) "TraceTypeQuery3" false 0 "ForDuration" false))
      (if _returnvalue_2
        (bind (_outhit_2 _returnvalue_3) (Collision|LineTraceByChannel (.Location (Collision|BreakHitResult _outhit)) (Transformation|GetWorldLocation (Variables|Character|GetMesh)) "TraceTypeQuery5" false 0 "ForDuration"))
        (if (not _returnvalue_3)
          (Variables|Default|SetHasTeleportAbility false)
          (Pawn|Components|CharacterMovement|DisableMovement (Variables|Character|GetCharacterMovement))
          (Input|DisableInput 0)
          (Utilities|FlowControl|Delay 2.0)
          (Input|EnableInput 0)
          (Pawn|Components|CharacterMovement|SetMovementMode (Variables|Character|GetCharacterMovement) "MOVE_Walking" 0)
          (Transformation|SetActorRotation (Math|Rotator|MakeRotfromX (- (.Location (Collision|BreakHitResult _outhit)) (Transformation|GetActorLocation))) true)
          (Transformation|SetActorLocation (.Location (Collision|BreakHitResult _outhit)) false true)
          (CallFunction|ResetKey1)
          (Components|Movement|StopMovementImmediately (Variables|Character|GetCharacterMovement)))))))

(fn ConstructionScript)